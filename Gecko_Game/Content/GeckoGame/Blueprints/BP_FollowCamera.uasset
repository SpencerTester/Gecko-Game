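; BP_FollowCamera is a camera Blueprint that computes confinement limits for an orthographic view, with no follow logic in the graphs shown.
; The construction script sizes the CameraConfines box from ConfinesExtent.
; On BeginPlay, GetCameraConfines derives min/max limits from the box bounds, inset by fractions of OrthoWidth.
; The minimum X and Y limits read the bounds' Y and Z components respectively, and Tick performs no work.
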(event EventBeginPlay
  (Utilities|GetCameraConfines
    (:Out
      (Utilities|FlowControl|Delay 0.0))))

(event EventTick
  (params (DeltaSeconds :type Float%20%28single-precision%29))
  (Variables|Default|SetDeltaSeconds DeltaSeconds))

(fn ConstructionScript
  (Components|Box|SetBoxExtent (Variables|Default|GetCameraConfines) (Variables|Default|GetConfinesExtent) true))